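; Notify_Move is an animation notify state that makes a boss advance toward its target during part of an animation.
; On begin, it finds the owner's BPC_Boss_Behavior component and has its AI controller issue a MoveToActor toward the component's TargetActor.
; On end, it stops the character's movement immediately.
; Both events return false without acting if the component or controller reference is invalid.
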(fn ReceivedNotifyBegin
  (params (MeshComp :type Skeletal%20Mesh%20Component%20Object%20Reference) (Animation :type Anim%20Sequence%20Base%20Object%20Reference) (TotalDuration :type Float%20%28single-precision%29) (EventReference :type Anim%20Notify%20Event%20Reference%20Structure%20%28by%20ref%29))
  (bind _returnvalue (Components|GetOwner MeshComp))
  (bind _returnvalue_2 (Actor|GetComponentbyClass _returnvalue "/Game/BossAIToolkit/Blueprints/BPC_Boss_Behavior.BPC_Boss_Behavior_C"))
  (bind _controllerref (Variables|/Game/BossAIToolkit/Blueprints/BPC_Boss_Behavior.BPC_Boss_Behavior_C|GetControllerRef _returnvalue_2))
  (Utilities|IsValid _returnvalue_2
    (:Is%20Valid
      (Utilities|IsValid _controllerref
        (:Is%20Valid
          (AI|Navigation|MovetoActor _controllerref (Variables|/Game/BossAIToolkit/Blueprints/BPC_Boss_Behavior.BPC_Boss_Behavior_C|GetTargetActor _returnvalue_2) -1.0 true true true 0)
          (return true))
        (:Is%20Not%20Valid
          _)))
    (:Is%20Not%20Valid
      _))
  (return false))

(fn ReceivedNotifyEnd
  (params (MeshComp :type Skeletal%20Mesh%20Component%20Object%20Reference) (Animation :type Anim%20Sequence%20Base%20Object%20Reference) (EventReference :type Anim%20Notify%20Event%20Reference%20Structure%20%28by%20ref%29))
  (bind _returnvalue (Components|GetOwner MeshComp))
  (bind _returnvalue_2 (Actor|GetComponentbyClass _returnvalue "/Game/BossAIToolkit/Blueprints/BPC_Boss_Behavior.BPC_Boss_Behavior_C"))
  (Utilities|IsValid _returnvalue_2
    (:Is%20Valid
      (Utilities|IsValid (Variables|/Game/BossAIToolkit/Blueprints/BPC_Boss_Behavior.BPC_Boss_Behavior_C|GetControllerRef _returnvalue_2)
        (:Is%20Valid
          (Components|Movement|StopMovementImmediately (Variables|/Script/Engine.Character|GetCharacterMovement (Variables|/Game/BossAIToolkit/Blueprints/BPC_Boss_Behavior.BPC_Boss_Behavior_C|GetCharacterRef _returnvalue_2)))
          (return true))
        (:Is%20Not%20Valid
          _)))
    (:Is%20Not%20Valid
      _))
  (return false))