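; BP_HellGateBullet is a projectile that flies toward the player, damaging on hit and exploding.
; At BeginPlay it randomly targets either the player's position or a random point in a flat area below it.
; A timeline lerps it there without sweeping, with a second track adding a vertical offset to the destination.
; Overlapping a "P"-tagged component applies point damage; either that or timeline completion spawns an explosion and destroys the actor.
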(event OnComponentBeginOverlap(Sphere)
  (params (OverlappedComponent :type Primitive%20Component%20Object%20Reference) (OtherActor :type Actor%20Object%20Reference) (OtherComp :type Primitive%20Component%20Object%20Reference) (OtherBodyIndex :type Integer) (bFromSweep :type Boolean) (SweepResult :type Hit%20Result%20Structure%20%28by%20ref%29))
  (bind (_bblockinghit _binitialoverlap _time _distance _location _impactpoint _normal _impactnormal) (Collision|BreakHitResult SweepResult))
  (if (Components|ComponentHasTag OtherComp "P")
    (Game|Damage|ApplyPointDamage OtherActor 2e+01 (* _impactnormal "-1.000000,-1.000000,-1.000000") SweepResult 0 0 "/Game/BossAIToolkit/Blueprints/DamageTypes/BP_DamageType_Default.BP_DamageType_Default_C")
    (Effects|SpawnEmitteratLocation "/Game/Particles/P_Explosion.P_Explosion" _impactpoint "0, 0, 0" "0.500000,0.500000,0.500000")
    (Actor|DestroyActor)))

(event EventBeginPlay
  (bind _returnvalue (Game|Player|GetPlayerPawn 0))
  (bind _returnvalue_2 (Transformation|GetActorLocation _returnvalue))
  (Variables|Default|SetTarget (Math|Vector|SelectVector (Math|Random|RandomPointinBoundingBox (- _returnvalue_2 "0.000000,0.000000,100.000000") "200.000000,200.000000,0.000000") _returnvalue_2 (Math|Random|RandomBool)))
  (Variables|Default|SetOriginalLocation (Transformation|GetActorLocation))
  (bind (_direction _新建轨道_0 _新建轨道_1) (Timeline|时间轴 Play)
    (:Update
      (Transformation|SetActorLocation (Math|Vector|Lerp(Vector) (Variables|Default|GetOriginalLocation) (+ (Variables|Default|GetTarget) (Math|Vector|Lerp(Vector) "0, 0, 0" "0.000000,0.000000,100.000000" _新建轨道_1)) _新建轨道_0) false false))
    (:Finished
      (Effects|SpawnEmitteratLocation "/Game/Particles/P_Explosion.P_Explosion" (Variables|Default|GetTarget) "0, 0, 0" "0.500000,0.500000,0.500000")
      (Actor|DestroyActor))))

(fn ConstructionScript)