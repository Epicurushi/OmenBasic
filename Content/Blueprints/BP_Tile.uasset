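; BP_Tile is a numbered tile that tracks open directions, apparently for procedural path generation.
; FindExit opens the side opposite the incoming direction and a random remaining exit; NewExit opens a further random one or reports none left.
; Both remove used sides from the possible-exits map and refresh arrow visibility from the directions map.
; Construction sets the debug label, arrows and foliage array; an event hides label and arrows in game.
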(event Custom|HideAllArrows
  (Development|SetHiddeninGame (Variables|Default|GetT_TileNumber) true true))

(event EventBeginPlay)

(event Collision|EventActorBeginOverlap
  (params (OtherActor :type Actor%20Object%20Reference)))

(event EventTick
  (params (DeltaSeconds :type Float%20%28single-precision%29)))

(fn ConstructionScript
  (Rendering|Components|TextRender|SetText (Variables|Default|GetT_TileNumber) (Utilities|Text|ToText(String) (Utilities|String|Append "Tile number is " (Utilities|String|ToString(Integer) (Variables|Default|GettileNumber)))))
  (CallFunction|ToggleArrows)
  (Variables|Default|Setfoliege (Utilities|Array|MakeArray (Variables|Default|GetFoliegeS) (Variables|Default|GetFoliegeW) (Variables|Default|GetFoliegeE) (Variables|Default|GetFoliegeN))))

(fn FindExit
  (params (incomeDirectionInterface :type E_Directions%20Enum :default "NewEnumerator0"))
  (bind _posibleexits (Variables|Default|GetPosibleExits))
  (Variables|Default|SetIncome%20Direction incomeDirectionInterface)
  (Utilities|Map|Add (Variables|Default|Getdirections) (.Value (Utilities|Map|Find (Variables|Default|GetOpositeDirection) (Variables|Default|GetIncome%20Direction))) true)
  (Utilities|Map|Remove _posibleexits (.Value (Utilities|Map|Find (Variables|Default|GetOpositeDirection) (Variables|Default|GetIncome%20Direction))))
  (bind _keys (Utilities|Map|Keys _posibleexits))
  (bind _output_get (Variables|Default|SetExit (.OutItem (Utilities|Array|Random _keys))))
  (Utilities|Map|Remove (Variables|Default|GetPosibleExits) _output_get)
  (Utilities|Map|Add (Variables|Default|Getdirections) (Variables|Default|GetExit) true)
  (CallFunction|ToggleArrows)
  (return (Variables|Default|GetExit)))

(fn NewExit
  (bind _posibleexits (Variables|Default|GetPosibleExits))
  (if (== (Utilities|Map|Length _posibleexits) 0)
    (CallFunction|ToggleArrows)
    (return true "NewEnumerator0")
    (else
      (bind _keys (Utilities|Map|Keys _posibleexits))
      (bind _output_get (Variables|Default|SetExit (.OutItem (Utilities|Array|Random _keys))))
      (Utilities|Map|Add (Variables|Default|Getdirections) _output_get true)
      (Utilities|Map|Remove (Variables|Default|GetPosibleExits) (Variables|Default|GetExit))
      (CallFunction|ToggleArrows)
      (return false (Variables|Default|GetExit)))))

(fn ToggleArrows
  (bind _keys (Utilities|Map|Keys (Variables|Default|Getdirections)))
  (for _array_element _keys
    (Rendering|SetVisibility (Utilities|Select :Index _array_element :NewEnumerator0 (Variables|Default|GetArrowNorth) :NewEnumerator1 (Variables|Default|GetArrowEast) :NewEnumerator2 (Variables|Default|GetArrowSouth) :NewEnumerator3 (Variables|Default|GetArrowWest)) (.Value (Utilities|Map|Find (Variables|Default|Getdirections) _array_element)) true))
  (return))