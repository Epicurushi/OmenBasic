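; BP_Trap is a spike trap that fires when a component tagged "P" overlaps its box while it is armed.
; It plays a mechanical warning sound, then after a short delay raises the spikes via a timeline and deals point damage to the player pawn if still inside.
; After a hold, the timeline reverses to lower the spikes, and the trap re-arms once that finishes.
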(event OnComponentBeginOverlap(Box)
  (params (OverlappedComponent :type Primitive%20Component%20Object%20Reference) (OtherActor :type Actor%20Object%20Reference) (OtherComp :type Primitive%20Component%20Object%20Reference) (OtherBodyIndex :type Integer) (bFromSweep :type Boolean) (SweepResult :type Hit%20Result%20Structure%20%28by%20ref%29))
  (if (and (Components|ComponentHasTag OtherComp "P") (not (Variables|Default|Gettriggered)))
    (Variables|Default|Settriggered true)
    (Audio|PlaySound2D "/Game/Sounds/Trap/94121__bmaczero__mechanical2_Cue.94121__bmaczero__mechanical2_Cue" 1.0 1.0 0.0 0 0)
    (Utilities|FlowControl|Delay 0.5)
    (Utilities|FlowControl|Sequence
      (:then_0
        (Audio|PlaySound2D "/Game/Sounds/Trap/443806__deathscyp__spiketrap.443806__deathscyp__spiketrap" 1.0 1.0 0.0 0 0))
      (:then_1
        (CallFunction|Attack)
        (for _array_element (Collision|GetOverlappingActors (Variables|Default|GetBox) "/Game/BossAIToolkit/Blueprints/Misc/BP_Player.BP_Player_C" :!class /Script/Engine.PrimitiveComponent)
          (if (== (.AsBP%20Player (Utilities|Casting|CastToBP_Player _array_element)) (.AsBP%20Player (Utilities|Casting|CastToBP_Player (Game|Player|GetPlayerPawn 0))))
            (Game|Damage|ApplyPointDamage (.AsBP%20Player (Utilities|Casting|CastToBP_Player _array_element)) 1e+02 (* (.ImpactNormal (Collision|BreakHitResult SweepResult)) "-1.000000,-1.000000,-1.000000") SweepResult 0 0 "/Game/BossAIToolkit/Blueprints/DamageTypes/BP_DamageType_Default.BP_DamageType_Default_C")))
        (Utilities|FlowControl|Delay 5.0)
        (CallFunction|Revert)))))

(event Custom|Attack
  (bind (_direction _newtrack_0) (Timeline|Timeline Play)
    (:Update
      (Transformation|SetRelativeLocation (Variables|Default|GetSpikes) (Math|Vector|Lerp(Vector) (Variables|Default|GetRelative%20Location) (+ (Variables|Default|GetRelative%20Location) "0.000000,0.000000,30.000000") _newtrack_0) false false))
    (:Finished
      (switch Utilities|FlowControl|Switch|SwitchonETimelineDirection _direction
        (:Backward
          (Variables|Default|Settriggered false))))))

(event Custom|Revert
  (bind (_direction _newtrack_0) (Timeline|Timeline ReverseFromEnd)
    (:Update
      (Transformation|SetRelativeLocation (Variables|Default|GetSpikes) (Math|Vector|Lerp(Vector) (Variables|Default|GetRelative%20Location) (+ (Variables|Default|GetRelative%20Location) "0.000000,0.000000,30.000000") _newtrack_0) false false))
    (:Finished
      (switch Utilities|FlowControl|Switch|SwitchonETimelineDirection _direction
        (:Backward
          (Variables|Default|Settriggered false))))))

(event EventBeginPlay
  (Variables|Default|SetRelative%20Location (Variables|/Script/Engine.SceneComponent|GetRelativeLocation (Variables|Default|GetSpikes))))

(fn ConstructionScript)