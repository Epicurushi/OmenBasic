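; Hell Gate is a stationary turret enemy with a pulsing red light and rotating core mesh.
; A tagged overlap in its sphere enables firing, swaps materials and fades in the player's combat music; exit reverses this.
; A looping timer spawns bullets when a player-to-core trace hits a "P"-tagged component.
; Damage shrinks the core with remaining health; death triggers an explosion, changes its tile's floor material and destroys the actor.
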(event OnComponentBeginOverlap(Sphere)
  (params (OverlappedComponent :type Primitive%20Component%20Object%20Reference) (OtherActor :type Actor%20Object%20Reference) (OtherComp :type Primitive%20Component%20Object%20Reference) (OtherBodyIndex :type Integer) (bFromSweep :type Boolean) (SweepResult :type Hit%20Result%20Structure%20%28by%20ref%29))
  ;[0.15 0.15 0.15 0.5] 进入战斗时防御塔发光，播放战斗音乐，退出攻击范围时淡出音乐并取消发光
  (if (Components|ComponentHasTag OtherComp "P")
    (Variables|Default|SetFire true)
    (Rendering|Material|SetMaterial (Variables|Default|GetStaticMesh) 0 "/Game/Materials/SigilMM_Inst3.SigilMM_Inst3")
    (Audio|Components|Audio|FadeIn (Variables|/Game/BossAIToolkit/Blueprints/Misc/BP_Player.BP_Player_C|GetActionMusic (.AsBP%20Player (Utilities|Casting|CastToBP_Player OtherActor))) 2.0 1.0 0.0 "Linear" :!class /Script/Engine.AudioComponent)))

(event OnComponentEndOverlap(Sphere)
  (params (OverlappedComponent :type Primitive%20Component%20Object%20Reference) (OtherActor :type Actor%20Object%20Reference) (OtherComp :type Primitive%20Component%20Object%20Reference) (OtherBodyIndex :type Integer))
  ;[0.15 0.15 0.15 0.5] 进入战斗时防御塔发光，播放战斗音乐，退出攻击范围时淡出音乐并取消发光
  (if (Components|ComponentHasTag OtherComp "P")
    (Variables|Default|SetFire false)
    (Rendering|Material|SetMaterial (Variables|Default|GetStaticMesh) 0 "/Game/Materials/SigilMM.SigilMM")
    (Audio|Components|Audio|FadeOut (Variables|/Game/BossAIToolkit/Blueprints/Misc/BP_Player.BP_Player_C|GetActionMusic (.AsBP%20Player (Utilities|Casting|CastToBP_Player (stale OnComponentBeginOverlap(Sphere) OtherActor)))) 3.0 0.0 "Linear" :!class /Script/Engine.AudioComponent)))

(event Custom|Hellgate%20Death
  (Effects|SpawnEmitteratLocation "/Game/Particles/P_Explosion.P_Explosion" (Transformation|GetActorLocation) "0, 0, 0" "5.000000,5.000000,5.000000")
  (Rendering|Material|SetMaterial (Variables|/Game/Blueprints/BP_Tile.BP_Tile_C|GetFloor (Variables|Default|GetTile)) 0 "/Game/Materials/Empty.Empty")
  (Actor|DestroyActor))

(event Custom|Shooty
  (if (Variables|Default|GetFire)
    (bind (_outhit _returnvalue) (Collision|LineTraceByChannel (Transformation|GetActorLocation (Game|Player|GetPlayerPawn 0)) (Transformation|GetWorldLocation (Variables|Default|GetStaticMesh1)) "TraceTypeQuery2" false 0 "None"))
    (if _returnvalue
      (if (Components|ComponentHasTag (.HitComponent (Collision|BreakHitResult _outhit)) "P")
        (Game|SpawnActorfromClass "/Game/Blueprints/Abilities/BP_HellGateBullet.BP_HellGateBullet_C" (Math|Transform|MakeTransform (Transformation|GetWorldLocation (Variables|Default|GetStaticMesh1)) "0, 0, 0" "1.000000,1.000000,1.000000") "Undefined" "MultiplyWithRoot" 0 0)
        (Audio|PlaySound2D "/Engine/VREditor/Sounds/UI/Dockable_Window_Close.Dockable_Window_Close" 1.0 1.0 0.0 0 0)))))

(event EventBeginPlay
  (bind _pointlight (Variables|Default|GetPointLight))
  (Components|Movement|SetUpdatedComponent (Variables|Default|GetRotatingMovement) (Variables|Default|GetStaticMesh1))
  (Variables|Default|SetCurrentHealth (Variables|Default|GetMaxHealth))
  (Variables|Default|SetOriginal%20Scale (Transformation|GetWorldScale (Variables|Default|GetStaticMesh1)))
  (Utilities|FlowControl|Sequence
    (:then_0
      (bind _lightalpha (Timeline|时间轴 PlayFromStart)
        (:Update
          (Rendering|Components|Light|SetLightColor _pointlight (Math|Color|Lerp(LinearColor) "(R=1.000000,G=0.000000,B=0.050000,A=1.000000)" "(R=1.000000,G=0.034813,B=0.000000,A=1.000000)" _lightalpha) true)
          (Rendering|Components|Light|SetIntensity _pointlight (Math|Float|Lerp 1.5e+02 1.8e+02 _lightalpha))
          (Rendering|Lighting|SetAttenuationRadius _pointlight (Math|Float|Lerp 7e+02 8e+02 _lightalpha)))))
    (:then_1
      (Utilities|Time|SetTimerbyEvent (delegate Custom|Shooty) 0.3 true))))

(event Game|Damage|EventAnyDamage
  (params (Damage :type Float%20%28single-precision%29) (DamageType :type Damage%20Type%20Object%20Reference) (InstigatedBy :type Controller%20Object%20Reference) (DamageCauser :type Actor%20Object%20Reference))
  (bind _original_scale (Variables|Default|GetOriginal%20Scale))
  (bind _output_get (Variables|Default|SetCurrentHealth (Math|Float|Clamp(Float) (- (Variables|Default|GetCurrentHealth) Damage) 0.0 (Variables|Default|GetMaxHealth))))
  (if (<= _output_get 0.0)
    (CallFunction|HellgateDeath)
    (else
      (Transformation|SetWorldScale3D (Variables|Default|GetStaticMesh1) (Math|Vector|Lerp(Vector) (/ _original_scale 5) _original_scale (/ (Variables|Default|GetCurrentHealth) (Variables|Default|GetMaxHealth)))))))

(fn ConstructionScript)