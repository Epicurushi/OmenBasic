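; Maze elevator that carries the player to the next procedurally generated level, unlocked by inventory item "i6".
; A tagged overlap consumes the item, spins the detached mechanism, blends the camera and animates four fences by timeline.
; Below 50 generator tiles, it spawns a larger BP_MazeGen above, rises on Tick, then restores the camera, destroys the previous maze and reverses the fences.
; Otherwise, it changes level to IceLevel.
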(event OnComponentBeginOverlap(Box)
  (params (OverlappedComponent :type Primitive%20Component%20Object%20Reference) (OtherActor :type Actor%20Object%20Reference) (OtherComp :type Primitive%20Component%20Object%20Reference) (OtherBodyIndex :type Integer) (bFromSweep :type Boolean) (SweepResult :type Hit%20Result%20Structure%20%28by%20ref%29))
  (bind _returnvalue (Game|GetGameMode))
  (bind _childactor (Variables|Default|GetChildActor))
  (bind _generator (Variables|Default|Getgenerator))
  (bind _childactor_2 (Variables|Default|GetChildActor))
  (bind _asbp_top_down_game_mode (Utilities|Casting|CastToBP_TopDownGameMode _returnvalue))
  (bind _childactor_3 (Variables|/Script/Engine.ChildActorComponent|GetChildActor _childactor))
  (bind _maxtiles (Variables|/Game/Blueprints/BP_MazeGen.BP_MazeGen_C|GetMaxTiles _generator))
  (bind _childactor_4 (Variables|/Script/Engine.ChildActorComponent|GetChildActor _childactor_2))
  (bind _generatorlevel (Variables|/Game/Blueprints/BP_MazeGen.BP_MazeGen_C|GetGeneratorLevel _generator))
  (bind _mazesize (Variables|/Game/Blueprints/BP_MazeGen.BP_MazeGen_C|GetMazeSize _generator))
  (bind _returnvalue_2 (+ _generatorlevel 12))
  (bind _returnvalue_3 (+ _mazesize 1))
  (bind _inventory (Variables|/Game/TopDown/Blueprints/BP_TopDownGameMode.BP_TopDownGameMode_C|GetInventory _asbp_top_down_game_mode))
  (bind _returnvalue_4 (Math|Random|RandomIntegerinRange 1 _returnvalue_2))
  (bind _returnvalue_5 (+ _maxtiles _returnvalue_4))
  (if (Components|ComponentHasTag OtherComp "P")
    (if (.ReturnValue (Utilities|Map|Find _inventory "i6"))
      (if (>= (Variables|/Game/Blueprints/BP_MazeGen.BP_MazeGen_C|GetMaxTiles (Variables|Default|Getgenerator)) 50)
        (Utilities|FlowControl|DoOnce false
          (:Completed
            (Collision|SetCollisionEnabled (Variables|Default|GetBox) "NoCollision")
            (Transformation|DetachFromActor _childactor_3 "KeepWorld" "KeepWorld" "KeepWorld")
            (Variables|/Script/Engine.RotatingMovementComponent|SetRotationRate (Variables|/Game/Blueprints/props/BP_ElevatorMechanism.BP_ElevatorMechanism_C|GetRotatingMovement (.AsBP%20Elevator%20Mechanism (Utilities|Casting|CastToBP_ElevatorMechanism _childactor_3))) "-60.000000,0.000000,0.000000")
            (Utilities|Map|Remove _inventory "i6")
            (Default|Updateinventory (Variables|/Game/TopDown/Blueprints/BP_TopDownGameMode.BP_TopDownGameMode_C|GetWG_Gameplay _asbp_top_down_game_mode) _inventory)
            (Audio|PlaySound2D "/Game/Sounds/Elevator/S_ElevatorUnlock.S_ElevatorUnlock" 1.0 1.0 0.0 0 0)
            (Utilities|FlowControl|Sequence
              (:then_0
                (Game|Player|SetViewTargetwithBlend (Game|GetPlayerController 0) self 3.0 "VTBlend_Linear" 0.0 false))
              (:then_1
                (CallFunction|StartAnimations)
                (Utilities|FlowControl|Delay 2.0)
                (bind _asbp_player (Utilities|Casting|CastToBP_Player (Game|GetPlayerCharacter 0)))
                (Default|ChangeLevel _asbp_player "IceLevel")))))
        (else
          (Utilities|FlowControl|DoOnce false
            (:Completed
              ;[0.15 0.15 0.15 0.5] L83修改
              (Collision|SetCollisionEnabled (Variables|Default|GetBox) "NoCollision")
              (Transformation|DetachFromActor _childactor_4 "KeepWorld" "KeepWorld" "KeepWorld")
              (Variables|/Script/Engine.RotatingMovementComponent|SetRotationRate (Variables|/Game/Blueprints/props/BP_ElevatorMechanism.BP_ElevatorMechanism_C|GetRotatingMovement (.AsBP%20Elevator%20Mechanism (Utilities|Casting|CastToBP_ElevatorMechanism _childactor_4))) "-60.000000,0.000000,0.000000")
              (Utilities|Map|Remove _inventory "i6")
              (Default|Updateinventory (Variables|/Game/TopDown/Blueprints/BP_TopDownGameMode.BP_TopDownGameMode_C|GetWG_Gameplay _asbp_top_down_game_mode) _inventory)
              (Audio|PlaySound2D "/Game/Sounds/Elevator/S_ElevatorUnlock.S_ElevatorUnlock" 1.0 1.0 0.0 0 0)
              (bind _output_get (Variables|Default|SetNewCenter (+ (Transformation|GetActorLocation) "0.000000,0.000000,2500.000000")))
              (Game|SpawnActorfromClass "/Game/Blueprints/BP_MazeGen.BP_MazeGen_C" (Math|Transform|MakeTransform _output_get "0, 0, 0" "1.000000,1.000000,1.000000") "Undefined" "MultiplyWithRoot" 0 true _returnvalue_5 800 (Math|Integer|SelectInt _mazesize _returnvalue_3 (< _returnvalue_5 (* _returnvalue_3 _returnvalue_3))) (+ (Variables|/Game/Blueprints/BP_MazeGen.BP_MazeGen_C|GetGeneratorLevel _generator) 1) self 0)
              (Utilities|FlowControl|Sequence
                (:then_0
                  (Game|Player|SetViewTargetwithBlend (Game|GetPlayerController 0) self 3.0 "VTBlend_Linear" 0.0 false))
                (:then_1
                  (CallFunction|StartAnimations)
                  (Utilities|FlowControl|Delay 2.0)
                  (Variables|Default|SettickCondition true)
                  (bind _returnvalue_6 (Audio|CreateSound2D "/Game/Sounds/Elevator/Elevator_Machine_Cue.Elevator_Machine_Cue" 1.0 1.0 0.0 0))
                  (bind _output_get_2 (Variables|Default|SetelevatorSound _returnvalue_6))
                  (Audio|Components|Audio|Play _output_get_2 0.0)))))))
      (else
        (Audio|PlaySound2D "/Game/Sounds/Elevator/S_ElevatorFail.S_ElevatorFail" 1.0 1.0 0.0 0 0)))))

(event Custom|StartAnimations
  (bind (_direction _newtrack_0) (Timeline|Timeline Play)
    (:Update
      (for _array_element (Utilities|Array|MakeArray (Variables|Default|Getfence) (Variables|Default|Getfence1) (Variables|Default|Getfence2) (Variables|Default|Getfence3))
        (Transformation|SetRelativeLocation _array_element (Math|Vector|MakeVector (.x (Variables|/Script/Engine.SceneComponent|GetRelativeLocation _array_element)) (.y (Variables|/Script/Engine.SceneComponent|GetRelativeLocation _array_element)) (Math|Float|Lerp (Variables|Default|GetOriginal%20Location%20Z) 0.0 _newtrack_0)) false false)))
    (:Finished
      (switch Utilities|FlowControl|Switch|SwitchonETimelineDirection _direction))))

(event Custom|fence%20down
  (bind _elevatorsound (Variables|Default|GetelevatorSound))
  (Audio|Components|Audio|Stop _elevatorsound)
  (Audio|Components|Audio|SetSound _elevatorsound "/Game/Sounds/Elevator/Elevator_End_Cue.Elevator_End_Cue")
  (Audio|Components|Audio|Play _elevatorsound 0.0)
  (bind (_direction _newtrack_0) (Timeline|Timeline ReverseFromEnd)
    (:Update
      (for _array_element (Utilities|Array|MakeArray (Variables|Default|Getfence) (Variables|Default|Getfence1) (Variables|Default|Getfence2) (Variables|Default|Getfence3))
        (Transformation|SetRelativeLocation _array_element (Math|Vector|MakeVector (.x (Variables|/Script/Engine.SceneComponent|GetRelativeLocation _array_element)) (.y (Variables|/Script/Engine.SceneComponent|GetRelativeLocation _array_element)) (Math|Float|Lerp (Variables|Default|GetOriginal%20Location%20Z) 0.0 _newtrack_0)) false false)))
    (:Finished
      (switch Utilities|FlowControl|Switch|SwitchonETimelineDirection _direction))))

(event EventBeginPlay
  (Variables|Default|SetOriginal%20Location%20Z (.z (Variables|/Script/Engine.SceneComponent|GetRelativeLocation (Variables|Default|Getfence))))
  (bind _output_get (Variables|Default|SetOriginalActorLocation (Transformation|GetActorLocation)))
  (Variables|Default|SettargetActorLocation (+ _output_get "0.000000,0.000000,2900.000000")))

(event Collision|EventActorBeginOverlap
  (params (OtherActor :type Actor%20Object%20Reference)))

(event EventTick
  (params (DeltaSeconds :type Float%20%28single-precision%29))
  (bind _returnvalue (Game|GetPlayerController 0))
  (if (Variables|Default|GettickCondition)
    (Transformation|SetActorLocation (Math|Interpolation|VInterptoConstant (Transformation|GetActorLocation) (Math|Vector|Lerp(Vector) (Variables|Default|GetOriginalActorLocation) (Variables|Default|GettargetActorLocation) (Variables|Default|GetmaxAlpha)) DeltaSeconds 3.5e+02) false false)
    (if (Utilities|Operators|EqualEqual (Transformation|GetActorLocation) (Variables|Default|GettargetActorLocation) 1e+01)
      (Variables|Default|SettickCondition false)
      (Game|Player|SetViewTargetwithBlend _returnvalue (Pawn|GetControlledPawn _returnvalue) 3.0 "VTBlend_Linear" 52.0 false)
      (Default|DestroyPreMaze (Variables|Default|Getgenerator))
      (CallFunction|FenceDown))))

(fn ConstructionScript)