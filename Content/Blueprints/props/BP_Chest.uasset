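; BP_Chest is a lootable maze chest that a player can open once inside its overlap sphere.
; Overlap registers the chest on BP_Player and enables Interact, which plays a sound, removes the label widget and runs a timeline.
; When the timeline finishes, it spawns one fixed and several random BP_Items, registering them with MazeGen for cleanup.
; BeginPlay scales the random item count by MazeGen's level and supports delayed debug auto-opening.
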(event OnComponentEndOverlap(Sphere)
  (params (OverlappedComponent :type Primitive%20Component%20Object%20Reference) (OtherActor :type Actor%20Object%20Reference) (OtherComp :type Primitive%20Component%20Object%20Reference) (OtherBodyIndex :type Integer))
  (if (Components|ComponentHasTag OtherComp "P")
    (Variables|Default|SetAble%20to%20Open false)))

(event OnComponentBeginOverlap(Sphere)
  (params (OverlappedComponent :type Primitive%20Component%20Object%20Reference) (OtherActor :type Actor%20Object%20Reference) (OtherComp :type Primitive%20Component%20Object%20Reference) (OtherBodyIndex :type Integer) (bFromSweep :type Boolean) (SweepResult :type Hit%20Result%20Structure%20%28by%20ref%29))
  (if (Components|ComponentHasTag OtherComp "P")
    (Development|PrintString "aaa")
    (bind _asbp_player (Utilities|Casting|CastToBP_Player OtherActor))
    (Variables|/Game/BossAIToolkit/Blueprints/Misc/BP_Player.BP_Player_C|Setinteract%20Chest _asbp_player self)
    (Variables|Default|SetAble%20to%20Open true)))

(event Custom|open)

(event EventBeginPlay
  (bind _widget (Variables|Default|GetWidget))
  (Utilities|IsValid (Variables|Default|GetMaze%20Gen)
    (:Is%20Valid
      (Variables|Default|SetMax%20Number%20of%20Items (Math|Random|RandomIntegerinRange 1 (+ (Variables|/Game/Blueprints/BP_MazeGen.BP_MazeGen_C|GetGeneratorLevel (Variables|Default|GetMaze%20Gen)) 1)))
      (Default|SetText (.AsWG%20Item%20World (Utilities|Casting|CastToWG_ItemWorld (UserInterface|GetWidget (Variables|Default|GetWidget)))) "Chest")
      (if (Variables|Default|GetDEBUG_AUTO_OPEN)
        (Utilities|FlowControl|Delay 1e+01)
        (Audio|PlaySound2D "/Game/Sounds/Chest/391947__ssierra1202__chest-openning-crack_Cue.391947__ssierra1202__chest-openning-crack_Cue" 1.0 1.0 0.0 0 0)
        (Development|SetHiddeninGame _widget true false)
        (Components|DestroyComponent _widget)
        (bind _newtrack_0 (Timeline|Timeline PlayFromStart)
          (:Update
            (Transformation|SetRelativeRotation (Variables|Default|GetStaticMesh1) "0, 0, 0" false false))
          (:Finished
            (bind _returnvalue (Game|SpawnActorfromClass "/Game/Blueprints/Items/BP_Items.BP_Items_C" (Math|Transform|MakeTransform (Transformation|GetActorLocation) "0, 0, 0" "1.000000,1.000000,1.000000") "Undefined" "MultiplyWithRoot" 0 "I5" 0))
            (Utilities|Array|Add (Variables|/Game/Blueprints/BP_MazeGen.BP_MazeGen_C|GetactorsToDestroy (Variables|Default|GetMaze%20Gen)) _returnvalue)
            (for _index (range 1 (Variables|Default|GetMax%20Number%20of%20Items))
              (bind _returnvalue_2 (Game|SpawnActorfromClass "/Game/Blueprints/Items/BP_Items.BP_Items_C" (Math|Transform|MakeTransform (Transformation|GetActorLocation) "0, 0, 0" "1.000000,1.000000,1.000000") "Undefined" "MultiplyWithRoot" 0 (Utilities|String|StringToName (Utilities|String|Append "I" (Utilities|String|ToString(Integer) (Math|Random|RandomIntegerinRange 1 5)))) 0))
              (Utilities|Array|Add (Variables|/Game/Blueprints/BP_MazeGen.BP_MazeGen_C|GetactorsToDestroy (Variables|Default|GetMaze%20Gen)) _returnvalue_2))))))
    (:Is%20Not%20Valid
      (Development|PrintText "HellERR_BP_Chest_MAZE_GEN_NOT_VALIDo"))))

(event EventInteract
  (bind _widget (Variables|Default|GetWidget))
  (if (and (Variables|Default|GetAble%20to%20Open) (not (Variables|Default|GetInteracting)))
    (Variables|Default|SetInteracting true)
    (Audio|PlaySound2D "/Game/Sounds/Chest/391947__ssierra1202__chest-openning-crack_Cue.391947__ssierra1202__chest-openning-crack_Cue" 1.0 1.0 0.0 0 0)
    (Development|SetHiddeninGame _widget true false)
    (Components|DestroyComponent _widget)
    (bind _newtrack_0 (Timeline|Timeline PlayFromStart)
      (:Update
        (Transformation|SetRelativeRotation (Variables|Default|GetStaticMesh1) "0, 0, 0" false false))
      (:Finished
        (bind _returnvalue (Game|SpawnActorfromClass "/Game/Blueprints/Items/BP_Items.BP_Items_C" (Math|Transform|MakeTransform (Transformation|GetActorLocation) "0, 0, 0" "1.000000,1.000000,1.000000") "Undefined" "MultiplyWithRoot" 0 "I5" 0))
        (Utilities|Array|Add (Variables|/Game/Blueprints/BP_MazeGen.BP_MazeGen_C|GetactorsToDestroy (Variables|Default|GetMaze%20Gen)) _returnvalue)
        (for _index (range 1 (Variables|Default|GetMax%20Number%20of%20Items))
          (bind _returnvalue_2 (Game|SpawnActorfromClass "/Game/Blueprints/Items/BP_Items.BP_Items_C" (Math|Transform|MakeTransform (Transformation|GetActorLocation) "0, 0, 0" "1.000000,1.000000,1.000000") "Undefined" "MultiplyWithRoot" 0 (Utilities|String|StringToName (Utilities|String|Append "I" (Utilities|String|ToString(Integer) (Math|Random|RandomIntegerinRange 1 5)))) 0))
          (Utilities|Array|Add (Variables|/Game/Blueprints/BP_MazeGen.BP_MazeGen_C|GetactorsToDestroy (Variables|Default|GetMaze%20Gen)) _returnvalue_2))))))

(fn ConstructionScript)